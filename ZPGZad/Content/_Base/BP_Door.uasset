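; BP_Door is an exit door that ends the game with a win screen once opened.
; A Box overlap opens it one time, only if the GameMode's IsUnlockedMessage returns true, with no filter on the overlapping actor.
; A Timeline curve lerps the actor's yaw through a swing.
; When it finishes, the door adds WBP_WinUI to the viewport and slows global time dilation to a near freeze.
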(event OnComponentBeginOverlap(Box)
  (params (OverlappedComponent :type Primitive%20Component%20Object%20Reference) (OtherActor :type Actor%20Object%20Reference) (OtherComp :type Primitive%20Component%20Object%20Reference) (OtherBodyIndex :type Integer) (bFromSweep :type Boolean) (SweepResult :type Hit%20Result%20Structure%20%28by%20ref%29))
  (if (not (Variables|Default|GetIsOpened))
    (bind _unlocked (Class|BPIIsUnlocked|IsUnlocked(Message) (Game|GetGameMode)))
    (if _unlocked
      (Variables|Default|SetIsOpened true)
      ;[1 1 1] Open Animation
      (bind _output_get (Variables|Default|SetStartRotation (Transformation|GetActorRotation)))
      (Variables|Default|SetTargetRotation (Math|Rotator|MakeRotator (.roll _output_get) (.pitch _output_get) (+ (.yaw _output_get) -7e+01)))
      (bind _opencurve (Timeline|Timeline PlayFromStart)
        (:Update
          (Transformation|SetActorRotation (Math|Rotator|Lerp(Rotator) (Variables|Default|GetStartRotation) (Variables|Default|GetTargetRotation) _opencurve)))
        (:Finished
          (bind _returnvalue (UserInterface|CreateWidget "/Game/_Base/WBP_WinUI.WBP_WinUI_C"))
          (UserInterface|Viewport|AddtoViewport _returnvalue 0)
          (Utilities|Time|SetGlobalTimeDilation 0.01))))))

(fn ConstructionScript)