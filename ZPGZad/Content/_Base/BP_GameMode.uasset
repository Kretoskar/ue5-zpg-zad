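; Game mode that tracks a collection objective and sets an unlocked flag once the target count is reached.
; On BeginPlay it runs a hardware benchmark and applies the resulting game user settings.
; Each Collect call increments the count and updates the player HUD, which also shows an all-collected message at or beyond the target.
; IsUnlocked exposes the flag to other objects.
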(event EventCollect
  (bind _returnvalue (Game|GetPlayerController 0))
  (bind _returnvalue_2 (HUD|GetHUD _returnvalue))
  (bind _output_get (Variables|Default|SetCurrentCount (+ (Variables|Default|GetCurrentCount) 1)))
  (Class|BPIUpdateCollectUI|UpdateCollectUI(Message) _returnvalue_2 _output_get)
  (Math|Integer|CompareInt _output_get (Variables|Default|GetTargetCount)
    (:>
      _)
    (:==
      _))
  (Variables|Default|SetUnlocked true)
  (Class|BPIonAllCollected|OnAllCollected(Message) _returnvalue_2))

(event EventBeginPlay
  (bind _returnvalue (Settings|GetGameUserSettings))
  (Class|GameUserSettings|RunHardwareBenchmark _returnvalue 10 1.0 1.0)
  (Class|GameUserSettings|ApplySettings _returnvalue true))

(fn ConstructionScript)

(fn IsUnlocked
  (return (Variables|Default|GetUnlocked)))